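; BP_Spikes is a spike hazard actor that reacts when the player moves quickly while overlapping it, currently only printing "Ouch" with no damage applied.
; Begin and end overlap with the player character open and close a Gate fed by Tick.
; While the gate is open, each tick casts the player pawn to MyCharacter and compares its capsule's physics linear velocity magnitude against a fixed threshold.
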(event EventBeginPlay)

(event EventTick
  (params (DeltaSeconds :type Float%20%28single-precision%29))
  ;[1 1 1] Is Player Overlapping?
  (Utilities|FlowControl|Gate true
    (:Exit
      ;[1 1 1] Check Movement Speed
      (bind _asmy_character (Utilities|Casting|CastToMyCharacter (Game|Player|GetPlayerPawn 0)))
      (bind _returnvalue (Physics|GetPhysicsLinearVelocity (Variables|/Script/Engine.Character|GetCapsuleComponent _asmy_character) "None"))
      (if (> (Math|Vector|VectorLength _returnvalue) 5e+02)
        (Development|PrintString "Ouch")))))

(event Collision|EventActorEndOverlap
  (params (OtherActor :type Actor%20Object%20Reference))
  ;[1 1 1] Is Player Overlapping?
  (if (== OtherActor (Game|GetPlayerCharacter 0))
    (Utilities|FlowControl|Gate true) ; enters at Close
  ))

(event Collision|EventActorBeginOverlap
  (params (OtherActor :type Actor%20Object%20Reference))
  ;[1 1 1] Is Player Overlapping?
  (if (== OtherActor (Game|GetPlayerCharacter 0))
    (Utilities|FlowControl|Gate true) ; enters at Open
  ))

(fn ConstructionScript)